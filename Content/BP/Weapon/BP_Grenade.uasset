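; BP_Grenade is a projectile grenade that explodes on its first hit or bounce.
; Both events share a DoOnce that stores the impact data and calls Boom for explosion effects, camera shake, radial damage and an impulse on the hit component.
; Boom also sprays randomly scaled, short-lived BP_DefaultProjectile shrapnel around the impact normal, then destroys the grenade after a brief delay.
; The impact decal logic is disconnected and never runs.
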(event `Boom`
  (bind _impact_point (`self.Impact Point`))
  (`GameplayStatics.SpawnEmitterAtLocation` "/Game/BallisticsVFX/Particles/Explosive/Explosion_GrenadeLauncher_1.Explosion_GrenadeLauncher_1" (`self.Location`) (`KismetMathLibrary.MakeRotFromZ` (* (`KismetMathLibrary.RandomUnitVectorInConeInRadians` (`KismetMathLibrary.GetDirectionUnitVector` (`self.Impact Normal`) (0.0 0.0 0.0)) (`self.Explosion Angle Variance VFX`)) -1.0)))
  (`GameplayStatics.PlayWorldCameraShake` "/Game/BP/Weapon/ExplosionShake.ExplosionShake_C" (`self.Location`) 0.0 5000.0)
  (`GameplayStatics.SpawnSoundAtLocation` "/Game/BallisticsVFX/SFX/Explodes/Explosions.Explosions" (`self.Location`) (struct) 0.75 0.0 0.0 "/Game/BallisticsVFX/SFX/Attentuations/Gun_Attenuation.Gun_Attenuation" null)
  (`GameplayStatics.ApplyRadialDamageWithFalloff` :`BaseDamage` 1000.0 :`MinimumDamage` 500.0 :`Origin` _impact_point :`DamageInnerRadius` 50.0 :`DamageOuterRadius` 500.0 :`DamageFalloff` 10.0 :`DamageCauser` null :`InstigatedByController` null)
  (`PrimitiveComponent.AddRadialImpulse` (`.HitComponent` (`GameplayStatics.BreakHitResult` (stale `self.SphereCollision.OnComponentHit` Hit))) _impact_point 500.0 1000000.0 "RIF_Linear" false)
  (for _ (range 26)
    (bind _returnvalue (`|SpawnActorFromClass` "/Game/BP/Weapon/BP_DefaultProjectile.BP_DefaultProjectile_C" (`KismetMathLibrary.MakeTransform` (`self.Location`) (`KismetMathLibrary.Conv_VectorToRotator` (`KismetMathLibrary.RandomUnitVectorInEllipticalConeInDegrees` (`self.Impact Normal`) 179.0 179.0)) (`KismetMathLibrary.MakeVector` (`KismetMathLibrary.RandomFloatInRange` 0.0 2.0) (`KismetMathLibrary.RandomFloatInRange` 0.0 2.0) (`KismetMathLibrary.RandomFloatInRange` 0.0 2.0))) "AdjustIfPossibleButAlwaysSpawn" "OverrideRootScale" null (`KismetMathLibrary.RandomFloatInRange` 1200.0 15000.0) null)) ; Spawn projectile
    (`self.SetLifeSpan` _returnvalue (`KismetMathLibrary.RandomFloatInRange` 1.0 3.0)))
  (`KismetSystemLibrary.Delay` 0.2)
  (`self.K2_DestroyActor`))

(event `self.SphereCollision.OnComponentHit`
  (params (HitComponent :type "PrimitiveComponent Object Reference") (OtherActor :type "Actor Object Reference") (OtherComp :type "PrimitiveComponent Object Reference") (NormalImpulse :type "Vector Structure") (Hit :type "HitResult Structure (by ref)"))
  (bind (_bblockinghit _binitialoverlap _time _distance _location _impactpoint _normal _impactnormal _physmat _hitactor _hitcomponent) (`GameplayStatics.BreakHitResult` Hit))
  (`/Engine/EditorBlueprintResources/StandardMacros.DoOnce` false :!label _label
    (:`Completed`
      (set `self.Location` _location)
      (set `self.Impact Point` _impactpoint)
      (set `self.Impact Normal` _impactnormal)
      (`self.Boom`))))

(event `self.ProjectileMovement.OnProjectileBounce`
  (params (ImpactResult :type "HitResult Structure (by ref)") (ImpactVelocity :type "Vector Structure (by ref)"))
  (goto _label))

(fn `UserConstructionScript`
  (`parent.UserConstructionScript`))