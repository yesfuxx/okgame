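; Default weapon projectile that shows a speed-based tracer and deals damage on impact.
; Tick activates the tracer flare at low speed, then, while it is active, scales the mesh by velocity.
; When movement stops, it pushes physics-simulating components with a clamped impulse, spawns BP_ImpactEffect and destroys itself.
; A second sequence branch damages BP_LittleGirl, doubled for head-bone hits, unless IsHelpGrenade is set.
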(event `self.ReceiveBeginPlay`)

(event `self.ReceiveTick`
  (params (DeltaSeconds :type "Float (single-precision)"))
  (bind _returnvalue (`KismetMathLibrary.VSize` (`MovementComponent.Velocity` (`self.ProjectileMovement`))))
  (bind _returnvalue_2 (`KismetMathLibrary.NormalizeToRange` _returnvalue 0.0 30000.0))
  ;[1 1 1] Tracer Scale per velocity + Tracer Flare
  (if (< _returnvalue_2 -1.0)
    _
    (elif (`ActorComponent.IsActive` (`self.TracerFlare`))
      (`SceneComponent.SetRelativeScale3D` (`self.Mesh`) (`KismetMathLibrary.Conv_DoubleToVector` (`KismetMathLibrary.MapRangeClamped` _returnvalue 0.0 10000.0 0.1 2.0)))
      (elif (<= _returnvalue_2 0.2)
        (`ActorComponent.Activate` (`self.TracerFlare`) false)))))

(event `Spawn FX`
  (`|SpawnActorFromClass` "/Game/BP/Effect/BP_ImpactEffect.BP_ImpactEffect_C" (`self.GetTransform` self) "Undefined" "OverrideRootScale" null (`self.Hit Result`) "NewEnumerator1" 100.0 true 20.0 (`self.ProjectileTransform`) 0.7 null))

(event `self.ProjectileMovement.OnProjectileStop`
  (params (ImpactResult :type "HitResult Structure (by ref)"))
  (bind _returnvalue (`Pawn.GetController` (`self.Instigator`)))
  (set `self.ProjectileTransform` (`SceneComponent.K2_GetComponentToWorld` (`self.SphereCollision`)))
  (bind _output_get (set `self.Hit Result` ImpactResult))
  (`|ExecutionSequence`
    (:`then_0`
      (bind (_bblockinghit _binitialoverlap _time _distance _location _impactpoint _normal _impactnormal _physmat _hitactor _hitcomponent _hitbonename) (`GameplayStatics.BreakHitResult` _output_get))
      (`/Engine/EditorBlueprintResources/StandardMacros.IsValid` _hitcomponent
        (:`Is Valid`
          (if (`SceneComponent.IsSimulatingPhysics` _hitcomponent "None")
            (`PrimitiveComponent.AddImpulseAtLocation` _hitcomponent (`KismetMathLibrary.ClampVectorSize` (* (`self.GetVelocity`) 1.0) 0.0 1000.0) _impactpoint "None")))
        (:`Is Not Valid`
          _))
      (`self.Spawn FX`)
      (`self.K2_DestroyActor`) ; Then destroy this projectile
    )
    (:`then_1`
      (if (not (`self.Is help Grenade`))
        (bind _asbp_little_girl (cast `/Game/BP/Character/BP_LittleGirl` _hitactor))
        (if (== _hitbonename "Head")
          (`GameplayStatics.ApplyDamage` _asbp_little_girl (* 2 (`self.Base Damage`)) _returnvalue self)
          (else
            (`GameplayStatics.ApplyDamage` _asbp_little_girl (`self.Base Damage`) _returnvalue self)))))))

(fn `UserConstructionScript`
  (`parent.UserConstructionScript`))