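; BP_PlayerState is a Blueprint that holds the player's score, health and death state.
; AddScore adds points to the score, and AddHP raises current HP without exceeding the maximum.
; CutHP lowers current HP, clamping it at zero and setting the Dead flag when it runs out.
; The event graph and construction script are empty, so all logic lives in these three functions.
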(fn `Add HP`
  (params (`Add HP Value` :type Integer))
  (bind _max_hp (`self.Max HP`))
  (bind _returnvalue (+ `Add HP Value` (`self.Current HP`)))
  (if (> _returnvalue _max_hp)
    (set `self.Current HP` _max_hp)
    (else
      (set `self.Current HP` _returnvalue))))

(fn `Add Score`
  (params (`A Score` :type Integer))
  (set `self.Player Score` (+ `A Score` (`self.Player Score`))))

(fn `Cut HP`
  (params (`Cut HP Value` :type Integer))
  (bind _returnvalue (- (`self.Current HP`) `Cut HP Value`))
  (if (<= _returnvalue 0)
    (set `self.Current HP` 0)
    (set `self.Dead` true)
    (else
      (set `self.Current HP` _returnvalue))))

(fn `UserConstructionScript`)