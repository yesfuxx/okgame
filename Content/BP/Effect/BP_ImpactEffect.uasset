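; Impact effect actor that plays surface-specific particles, decals and sound at a projectile hit.
; BeginPlay unpacks HitResult and finds the surface's DT_Material row, falling back to a default.
; It spawns an emitter scaled by size and impact speed, randomized fading decals, and sound pitched by time dilation.
; Ttttttt adds rear-spatter decals at the impact and along a forward trace, while the cone-traced SpawnSplatter is only called from disconnected logic.
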(event `self.ReceiveBeginPlay`
  (bind (_bblockinghit _binitialoverlap _time _distance _location _impactpoint _normal _impactnormal _physmat _hitactor _hitcomponent _hitbonename) (`GameplayStatics.BreakHitResult` (`self.Hit Result`)))
  (set `self.SurfaceType Feedback` (`PhysicalMaterial.SurfaceType` _physmat))
  (set `self.Impact Point` _impactpoint)
  (set `self.Impact Normal` _impactnormal)
  (set `self.Hit Component` _hitcomponent)
  (set `self.Hit Actor` _hitactor)
  (set `self.Hit Bone` _hitbonename)
  (`self.Get FX Type`))

(event `Get FX Type`
  (bind _returnvalue (`|GetDataTableRow` "/Game/BP/Effect/DT_Material.DT_Material" (`|GetEnumeratorName` (`self.SurfaceType Feedback`)))
    (:`then`
      (set `self.Material Values` _returnvalue))
    (:`RowNotFound`
      (bind _returnvalue_2 (`|GetDataTableRow` "/Game/BP/Effect/DT_Material.DT_Material" "SurfaceType_Default")
        (:`then`
          _)
        (:`RowNotFound`
          _))
      (set `self.Material Values` _returnvalue_2)))
  (`self.Spawn `)
  (`KismetSystemLibrary.PrintString` (`KismetSystemLibrary.GetDisplayName` (`.RearSpatterDecal_27_B70030244A483D74E6F9C79AB926F68E` (break `/Game/BP/Effect/S_MaterialData` (`self.Material Values`)))) true true (struct :`R` 0.831012 :`G` 0.074322 :`B` 1.0 :`A` 1.0)))

(event `Spawn`
  (`|ExecutionSequence`
    (:`then_0`
      (bind _returnvalue (`GameplayStatics.SpawnEmitterAtLocation` (`.ImpactParticleFX_15_C7070D4D4A3BEB78890DC4B4977D0D1F` (break `/Game/BP/Effect/S_MaterialData` (`self.Material Values`))) (`self.Impact Point`) (`KismetMathLibrary.MakeRotFromZ` (`self.Impact Normal`))))
      (bind _output_get (set `self.Main FX Emitter` _returnvalue))
      (`SceneComponent.SetRelativeScale3D` _output_get (* (select `/Game/BP/Effect/E_ProjectileSIze` (`self.FXSize`) :`NewEnumerator0` (0.8 0.8 0.8) :`NewEnumerator1` (1.0 1.0 1.0) :`NewEnumerator2` (1.5 1.5 1.5) :!type "Vector Structure") (* (`KismetMathLibrary.MapRangeClamped` (`self.Impact Speed`) (`self.NormalisedRangeMin`) (`self.NormalisedRangeMax`) 0.4 1.0) (`self.ImpactForceMultiplier`))))
      (`self.Spawn Decals`))
    (:`then_1`
      (`self.ttttttt`))))

(event `Spawn Decals`
  (bind _decal_life (`self.Decal Life`))
  (bind _decal_life_2 (`self.Decal Life`))
  (bind (_surface _impactparticlefx _impactsound _impactdecal _decalsize) (break `/Game/BP/Effect/S_MaterialData` (`self.Material Values`)))
  (bind _returnvalue (`KismetMathLibrary.MakeRotator` (`KismetMathLibrary.RandomFloatInRange` 0.0 360.0) (.pitch (`KismetMathLibrary.Conv_VectorToRotator` (* (`self.Impact Normal`) -1))) (.yaw (`KismetMathLibrary.Conv_VectorToRotator` (* (`self.Impact Normal`) -1)))))
  (bind _returnvalue_2 (* (select `/Game/BP/Effect/E_ProjectileSIze` (`self.FXSize`) :`NewEnumerator0` (0.8 0.8 0.8) :`NewEnumerator1` (1.0 1.0 1.0) :`NewEnumerator2` (1.5 1.5 1.5) :!type "Vector Structure") (* (`KismetMathLibrary.MakeVector` (.x _decalsize) (.y _decalsize) (.z _decalsize)) (`KismetMathLibrary.RandomFloatInRange` 0.75 1.9))))
  (bind _returnvalue_3 (`KismetMaterialLibrary.CreateDynamicMaterialInstance` (`.ImpactDecal_18_6A83F1574EBF9E995754BFBD63951ACB` (break `/Game/BP/Effect/S_MaterialData` (`self.Material Values`)))))
  (bind _output_get (set `self.Impact Decal Mat` _returnvalue_3))
  (`/Engine/EditorBlueprintResources/StandardMacros.IsValid` _output_get
    (:`Is Valid`
      (`MaterialInstanceDynamic.SetScalarParameterValue` _output_get "Frame" (`KismetMathLibrary.Conv_IntToDouble` (`KismetMathLibrary.RandomIntegerInRange` 0 3)))
      (if (`self.Decals Attached?`)
        (bind _returnvalue_4 (`GameplayStatics.SpawnDecalAttached` (`self.Impact Decal Mat`) _returnvalue_2 (`self.Hit Component`) (`self.Hit Bone`) (`self.Impact Point`) _returnvalue "KeepWorldPosition" _decal_life))
        (`/Engine/EditorBlueprintResources/StandardMacros.IsValid` _returnvalue_4
          (:`Is Valid`
            (`DecalComponent.SetFadeOut` _returnvalue_4 _decal_life 5.0 false))
          (:`Is Not Valid`
            _))
        (else
          (bind _returnvalue_5 (`GameplayStatics.SpawnDecalAtLocation` (`self.Impact Decal Mat`) _returnvalue_2 (`self.Impact Point`) _returnvalue _decal_life_2))
          (`/Engine/EditorBlueprintResources/StandardMacros.IsValid` _returnvalue_5
            (:`Is Valid`
              (`DecalComponent.SetFadeOut` _returnvalue_5 _decal_life_2 5.0 false))
            (:`Is Not Valid`
              _))))
      (`self.SpawnSounds`))))

(event `Spawn Splatter`
  (bind _impact_point (`self.Impact Point`))
  (bind (_projectile_transform_location _projectile_transform_rotation) (`KismetMathLibrary.BreakTransform` (`self.Projectile Transform`)))
  (bind (_surface _impactparticlefx _impactsound _impactdecal _decalsize _particledecal _rearspatterdecal) (break `/Game/BP/Effect/S_MaterialData` (`self.Material Values`)))
  (`/Engine/EditorBlueprintResources/StandardMacros.IsValid` _rearspatterdecal
    (:`Is Valid`
      (bind (_outhit _returnvalue) (`KismetSystemLibrary.LineTraceSingle` _impact_point (+ _impact_point (* (`KismetMathLibrary.RandomUnitVectorInEllipticalConeInDegrees` (`KismetMathLibrary.GetForwardVector` _projectile_transform_rotation) 10.0 10.0) 500.0)) "TraceTypeQuery1" false (`|MakeArray` (`self.Hit Actor`)) "Persistent"))
      (if _returnvalue
        (bind (_bblockinghit _binitialoverlap _time _distance _location _impactpoint _normal _impactnormal _physmat _hitactor _hitcomponent) (`GameplayStatics.BreakHitResult` _outhit))
        (`|GetDataTableRow` "/Game/BP/Effect/DT_Material.DT_Material" (`|GetEnumeratorName` (`PhysicalMaterial.SurfaceType` _physmat))
          (:`then`
            (bind _returnvalue_2 (`KismetMaterialLibrary.CreateDynamicMaterialInstance` _rearspatterdecal))
            (bind _output_get (set `self.Splatter Decal Mat` _returnvalue_2))
            (`/Engine/EditorBlueprintResources/StandardMacros.IsValid` _output_get
              (:`Is Valid`
                (`MaterialInstanceDynamic.SetScalarParameterValue` _output_get "Frame" (`KismetMathLibrary.RandomFloatInRange` 0.0 4.0))
                (`MaterialInstanceDynamic.SetScalarParameterValue` _returnvalue_2 "Frame" (`KismetMathLibrary.RandomFloatInRange` 0.0 4.0))
                (bind _returnvalue_3 (`GameplayStatics.SpawnDecalAttached` _returnvalue_2 (* (* (`KismetMathLibrary.MakeVector` (.x (3.0 10.0 10.0)) (.y (3.0 10.0 10.0)) (.z (3.0 10.0 10.0))) (`KismetMathLibrary.RandomFloatInRange` 1.5 3.5)) (select `byte` (`self.FXSize`) :`0` (0.0 0.0 0.0) :`1` (0.0 0.0 0.0) :`2` (0.0 0.0 0.0) :!type "Vector Structure")) _hitcomponent "None" _location (`KismetMathLibrary.MakeRotator` (`KismetMathLibrary.RandomFloatInRange` 0.0 360.0) (.pitch (`KismetMathLibrary.Conv_VectorToRotator` (* _normal -1))) (.yaw (`KismetMathLibrary.Conv_VectorToRotator` (* _normal -1)))) "KeepWorldPosition" (`self.Decal Life`)))
                (`/Engine/EditorBlueprintResources/StandardMacros.IsValid` _returnvalue_3
                  (:`Is Valid`
                    (`DecalComponent.SetFadeOut` _returnvalue_3 (`self.Decal Life`) 5.0 false)))))))))))

(event `SpawnSounds`
  (`GameplayStatics.SpawnSoundAtLocation` (`.ImpactSound_13_076BE65B48FEAB2283ED58B91393C0F7` (break `/Game/BP/Effect/S_MaterialData` (`self.Material Values`))) (`self.Impact Point`) (struct) 0.75 (`GameplayStatics.GetGlobalTimeDilation`) 0.0 null null))

(event `ttttttt`
  (bind _decal_life (`self.Decal Life`))
  (bind (_projectile_transform_location _projectile_transform_rotation) (`KismetMathLibrary.BreakTransform` (`self.Projectile Transform`)))
  (bind _impact_point (`self.Impact Point`))
  (bind _decal_life_2 (`self.Decal Life`))
  (bind (_surface _impactparticlefx _impactsound _impactdecal _decalsize _particledecal _rearspatterdecal) (break `/Game/BP/Effect/S_MaterialData` (`self.Material Values`)))
  (bind (_surface_2 _impactparticlefx_2 _impactsound_2 _impactdecal_2 _decalsize_2) (break `/Game/BP/Effect/S_MaterialData` (`self.Material Values`)))
  (`/Engine/EditorBlueprintResources/StandardMacros.IsValid` _rearspatterdecal
    (:`Is Valid`
      (bind _returnvalue (`KismetMaterialLibrary.CreateDynamicMaterialInstance` _rearspatterdecal))
      (`/Engine/EditorBlueprintResources/StandardMacros.IsValid` _returnvalue
        (:`Is Valid`
          (bind _output_get (set `self.Impact Decal Mat` _returnvalue))
          (`MaterialInstanceDynamic.SetScalarParameterValue` _output_get "Frame" (`KismetMathLibrary.Conv_IntToDouble` (`KismetMathLibrary.RandomIntegerInRange` 0 3)))
          (bind _returnvalue_2 (`GameplayStatics.SpawnDecalAtLocation` (`self.Impact Decal Mat`) (* (select `/Game/BP/Effect/E_ProjectileSIze` (`self.FXSize`) :`NewEnumerator0` (0.8 0.8 0.8) :`NewEnumerator1` (1.0 1.0 1.0) :`NewEnumerator2` (1.5 1.5 1.5) :!type "Vector Structure") (* (`KismetMathLibrary.MakeVector` (.x _decalsize_2) (.y _decalsize_2) (.z _decalsize_2)) (`KismetMathLibrary.RandomFloatInRange` 0.75 1.9))) (`self.Impact Point`) (`KismetMathLibrary.MakeRotator` (`KismetMathLibrary.RandomFloatInRange` 0.0 360.0) (.pitch (`KismetMathLibrary.Conv_VectorToRotator` (* (`self.Impact Normal`) -1))) (.yaw (`KismetMathLibrary.Conv_VectorToRotator` (* (`self.Impact Normal`) -1)))) _decal_life_2))
          (`/Engine/EditorBlueprintResources/StandardMacros.IsValid` _returnvalue_2
            (:`Is Valid`
              (`DecalComponent.SetFadeOut` _returnvalue_2 _decal_life_2 5.0 false)
              (bind _outhit (`KismetSystemLibrary.LineTraceSingle` _impact_point (+ _impact_point (* (`KismetMathLibrary.GetForwardVector` _projectile_transform_rotation) 500.0)) "TraceTypeQuery1" false (`|MakeArray` (`self.Hit Actor`)) "None" true (struct :`R` 1.0 :`A` 1.0) (struct :`G` 1.0 :`A` 1.0) 2.0))
              (bind (_bblockinghit _binitialoverlap _time _distance _location _impactpoint _normal _impactnormal) (`GameplayStatics.BreakHitResult` _outhit))
              (bind _returnvalue_3 (`GameplayStatics.SpawnDecalAtLocation` (`self.Impact Decal Mat`) (* (* (`KismetMathLibrary.MakeVector` (.x (3.0 10.0 10.0)) (.y (3.0 10.0 10.0)) (.z (3.0 10.0 10.0))) (`KismetMathLibrary.RandomFloatInRange` 1.5 3.5)) (select `byte` (`self.FXSize`) :`0` (0.0 0.0 0.0) :`1` (0.0 0.0 0.0) :`2` (0.0 0.0 0.0) :!type "Vector Structure")) _location (`KismetMathLibrary.MakeRotator` (`KismetMathLibrary.RandomFloatInRange` 0.0 360.0) (.pitch (`KismetMathLibrary.Conv_VectorToRotator` (* _impactnormal -1))) (.yaw (`KismetMathLibrary.Conv_VectorToRotator` (* _impactnormal -1)))) _decal_life))
              (`/Engine/EditorBlueprintResources/StandardMacros.IsValid` _returnvalue_3
                (:`Is Valid`
                  (`DecalComponent.SetFadeOut` _returnvalue_3 _decal_life 5.0 false))))))))))

(fn `UserConstructionScript`
  (set `self.bAutoDestroyWhenFinished` true))